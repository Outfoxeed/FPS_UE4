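; Game manager for Dive In Hell that registers with the GameInstance, driving fall progression and the enemy/platform cycle.
; Tick accumulates distance and ramps fall speed over level time after a grace period; delays scale along the same curve.
; Scoring triggers delayed enemy spawning and a warning; rotating toward enemies clears it and schedules a platform warning.
; Rotating upward then spawns a platform, with CanPlayerRotate true only while a warning exists.
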(event Custom|OnScoreAdded
  (bind _enemyspawner (Variables|Default|GetEnemySpawner))
  ;[1 0.8194 0] Score added
  (Utilities|IsValid _enemyspawner
    (:Is%20Valid
      (bind _fightduration (CallFunction|LerpwithGameTime (Variables|Fight|GetTimeBeforeEnemySpawnMinMax)))
      (Utilities|FlowControl|Delay _fightduration)
      (Class|EnemySpawner|SpawnEnemiesInstant _enemyspawner)
      (CallFunction|TriggerEnemyWarning))
    (:Is%20Not%20Valid
      (Development|PrintString "Couldn't get EnemySpawner"))))

(event Custom|TriggerPlatformWarning
  ;[0.3646 0 0.004144] Warnings
  (bind _returnvalue (UserInterface|CreateWidget (Variables|Warnings|GetPlatformWarningClass)))
  (bind _output_get (Variables|Warnings|SetPlatformWarning _returnvalue))
  (UserInterface|Viewport|AddtoViewport _output_get 0))

(event Custom|TriggerEnemyWarning
  ;[0.3646 0 0.004144] Warnings
  (bind _returnvalue (UserInterface|CreateWidget (Variables|Warnings|GetEnemyWarningClass)))
  (bind _output_get (Variables|Warnings|SetEnemyWarning _returnvalue))
  (UserInterface|Viewport|AddtoViewport _returnvalue 0))

(event Custom|OnPlayerRotate
  (params (NewPlayerWatchingUp :type Boolean))
  ;[1 0.8194 0] Score added
  (if (and (not NewPlayerWatchingUp) (Utilities|IsValid (Variables|Warnings|GetEnemyWarning)))
    ;;[1 1 1] The player is rotating towards enemy -> remove enemy warning + Prepare to trigger platform warning
    (Widget|RemovefromParent (Variables|Warnings|GetEnemyWarning))
    (Variables|Warnings|SetEnemyWarning 0)
    (Development|PrintString "Remove enemy wrning")
    (bind _fightduration (CallFunction|LerpwithGameTime (Variables|Fight|GetFightDurationMinMax)))
    (Utilities|FlowControl|Delay _fightduration)
    (CallFunction|TriggerPlatformWarning)
    (elif (and NewPlayerWatchingUp (Utilities|IsValid (Variables|Warnings|GetPlatformWarning)))
      ;;[1 1 1] The player is rotating towars platform -> remove platform warning + spawn platform
      (Widget|RemovefromParent (Variables|Warnings|GetPlatformWarning))
      (Variables|Warnings|SetPlatformWarning 0)
      (Development|PrintString "Remove platform warning")
      (Default|SpawnPlatform (Variables|Default|GetPlatformsSpawner))
      (else
        (Development|PrintString "No Warning to remove")))))

(event Custom|InstantPlayerDeath
  (Default|Die (Variables|Default|GetFirstPersonCharacter)))

(event EventTick
  (params (DeltaSeconds :type Float%20%28single-precision%29))
  (bind _speedminmax (Variables|Default|GetSpeedMinMax))
  (bind (_x _y) (Math|Vector2D|BreakVector2D _speedminmax))
  (Default|IncreaseDistanceTravelled (Variables|Default|GetGameInstance) DeltaSeconds)
  ;[0 1 0.01445] Increase Fall Speed
  (Variables|/Game/DiveInHell_GameInstanceBP.DiveInHell_GameInstanceBP_C|SetFallSpeed (Variables|Default|GetGameInstance) (Math|Float|Lerp _x _y (Math|Float|Clamp(Float) (/ (- (Actor|GetGameTimeSinceCreation) (Variables|Default|GetTimeWithoutAcceleration)) (- (Variables|Default|GetLevelDuration) (Variables|Default|GetTimeWithoutAcceleration)))))))

(event EventBeginPlay
  (Utilities|FlowControl|Sequence
    (:then_0
      ;[1 1 1] Set GameInstance's GameManager
      (bind _asdive_in_hell_game_instance_bp (Utilities|Casting|CastToDiveInHell_GameInstanceBP (Game|GetGameInstance)))
      (bind _output_get (Variables|Default|SetGameInstance _asdive_in_hell_game_instance_bp))
      (Variables|/Game/DiveInHell_GameInstanceBP.DiveInHell_GameInstanceBP_C|SetGameManager _output_get self))
    (:then_1
      ;[1 1 1] Get FirstPersonCharacter
      (bind _asfirst_person_character (Utilities|Casting|CastToFirstPersonCharacter (Game|GetPlayerCharacter 0)))
      (Variables|Default|SetFirstPersonCharacter _asfirst_person_character))))

(fn ConstructionScript)

(fn LerpwithGameTime
  (params (MinMax :type Vector%202D%20Structure))
  (bind (_x _y) (Math|Vector2D|BreakVector2D MinMax))
  (return (Math|Float|Lerp _x _y (Math|Float|Clamp(Float) (/ (- (Actor|GetGameTimeSinceCreation) (Variables|Default|GetTimeWithoutAcceleration)) (- (Variables|Default|GetLevelDuration) (Variables|Default|GetTimeWithoutAcceleration)))))))

(fn CanPlayerRotate
  (return (or (Utilities|IsValid (Variables|Warnings|GetEnemyWarning)) (Utilities|IsValid (Variables|Warnings|GetPlatformWarning)))))