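; Enemy actor that follows the player, damages them on contact and can be killed.
; On BeginPlay its AI controller runs NewBehaviorTree, meant to drive the chase.
; A hit on a FirstPersonCharacter applies damage to that character.
; EnemyTakesDamage lowers EnemyHealth by one per call and destroys the actor once it reaches zero.
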(event EventBeginPlay
  ;[1 1 1] Make Enemy follow player
  (AI|RunBehaviorTree (AI|GetAIController self) "/Game/behavior/NewBehaviorTree.NewBehaviorTree"))

(event Collision|EventHit
  (params (MyComp :type Primitive%20Component%20Object%20Reference) (Other :type Actor%20Object%20Reference) (OtherComp :type Primitive%20Component%20Object%20Reference) (bSelfMoved :type Boolean) (HitLocation :type Vector :default "0, 0, 0") (HitNormal :type Vector :default "0, 0, 0") (NormalImpulse :type Vector :default "0, 0, 0") (Hit :type Hit%20Result%20Structure%20%28by%20ref%29))
  (bind _hitactor (Collision|BreakHitResult Hit))
  ;[1 1 1] Apply damage to player
  (Utilities|Casting|CastToFirstPersonCharacter _hitactor)
  (Game|Damage|ApplyDamage _hitactor 1.0 0 self))

(fn ConstructionScript)

(fn EnemyTakesDamage
  (if (> (Variables|Default|GetEnemyHealth) 0)
    (Variables|Default|SetEnemyHealth (- (Variables|Default|GetEnemyHealth) 1))
    (if (== (Variables|Default|GetEnemyHealth) 0)
      (Actor|DestroyActor)
      (else
        (return)))
    (else
      (Actor|DestroyActor))))